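; Enemy spawner actor that makes a single timed attempt to spawn an enemy near itself.
; BeginPlay starts a non-looping SpawnTime timer, which spawns only if the Enemy_base actor count is below MaxEnemies.
; SpawnEnemy creates an Enemy_base running BT_EnemyBehavior at a random reachable navigation point within a fixed radius of the spawner.
; The timer is never re-armed in these graphs.
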(event Custom|TryToSpawnEnemy
  (bind _outactors (Actor|GetAllActorsOfClass "/Game/Enemy/Enemy_base.Enemy_base_C"))
  (if (< (Utilities|Array|Length _outactors) (Variables|Default|GetMaxEnemies))
    (Utilities|SpawnEnemy)))

(event EventBeginPlay
  (Utilities|Time|SetTimerbyEvent (delegate Custom|TryToSpawnEnemy) (Variables|Default|GetSpawnTime)))

(event Collision|EventActorBeginOverlap
  (params (OtherActor :type Actor%20Object%20Reference)))

(event EventTick
  (params (DeltaSeconds :type Float%20%28single-precision%29)))

(fn ConstructionScript)