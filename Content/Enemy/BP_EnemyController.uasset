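; Enemy AI controller that runs the enemy behavior tree and lets enemies react to noises.
; On BeginPlay it starts BT_EnemyBehavior.
; When PawnSensing hears a noise within HearingDistance of the controlled pawn, UpdateSoundBB writes the location and a heard-sound flag to the blackboard.
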(event OnHearNoise(PawnSensing)
  (params (Instigator :type Pawn%20Object%20Reference) (Location :type Vector%20%28by%20ref%29 :default "0, 0, 0") (Volume :type Float%20%28single-precision%29))
  (if (< (Math|Vector|VectorLength (- Location (Transformation|GetActorLocation (Pawn|GetControlledPawn)))) (Variables|Default|GetHearingDistance))
    (Utilities|UpdateSoundBB Location)))

(event EventBeginPlay
  (AI|RunBehaviorTree "/Game/Enemy/BT_EnemyBehavior.BT_EnemyBehavior"))

(event EventTick
  (params (DeltaSeconds :type Float%20%28single-precision%29)))

(fn ConstructionScript)