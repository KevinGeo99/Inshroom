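; BP_Minion is a companion pawn that follows the player's BP_Mush_PlayerB and takes Follow, Wait and Move There commands.
; Following starts on BeginPlay or on seeing the player, gated by a bool and distance check, then reissues AI MoveTo every 0.2 seconds while Follow Me is active.
; Wait and MoveThere switch the active command to halt or head to a location.
; Its sphere overlap damages actors tagged Enemy_base.
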(event OnComponentBeginOverlap(Sphere)
  (params (OverlappedComponent :type Primitive%20Component%20Object%20Reference) (OtherActor :type Actor%20Object%20Reference) (OtherComp :type Primitive%20Component%20Object%20Reference) (OtherBodyIndex :type Integer) (bFromSweep :type Boolean) (SweepResult :type Hit%20Result%20Structure%20%28by%20ref%29))
  ;[1 1 1] Collision_Damage
  (if (Actor|ActorHasTag OtherActor "Enemy_base")
    (Game|Damage|ApplyDamage OtherActor 2e+01 0 self "/Script/Engine.DamageType")))

(event OnSeePawn(PawnSensing)
  (params (Pawn :type Pawn%20Object%20Reference))
  (Utilities|Casting|CastToBP_Mush_PlayerB Pawn)
  (CallFunction|FollowPlayer self))

(event Custom|Follow%20Player
  ;[1 1 1] Follow_player
  (if (Variables|Default|GetFollowPlayer?)
    (if (>= (Transformation|GetDistanceTo (Variables|Default|GetChar%20REF)) 4e+02)
      (AI|AIMoveTo self "0, 0, 0" (Variables|Default|GetChar%20REF) 1.5e+02 false :!label _label
        (:then
          (Utilities|FlowControl|Delay 0.2 :!label _label_2)
          (switch Utilities|FlowControl|Switch|SwitchonMinion_commands (Variables|Default|GetActive%20Command)
            (:NewEnumerator0
              (goto _label)))))
      (else
        (AI|AIMoveTo self "0, 0, 0" self 1.5e+02 false
          (:then
            (goto _label_2)))))))

(event Custom|Wait
  ;[1 1 1] Wait_Commands
  (Variables|Default|SetActive%20Command "NewEnumerator1")
  (Class|NavMovementComponent|StopActiveMovement (Variables|Character|GetCharacterMovement)))

(event Custom|Stop%20Movements
  ;[1 1 1] Follow_player
  (AI|AIMoveTo self "0, 0, 0" self 1.5e+02 false
    (:then
      (Utilities|FlowControl|Delay 0.2 :!label _label)
      (switch Utilities|FlowControl|Switch|SwitchonMinion_commands (Variables|Default|GetActive%20Command)
        (:NewEnumerator0
          (AI|AIMoveTo self "0, 0, 0" (Variables|Default|GetChar%20REF) 1.5e+02 false
            (:then
              (goto _label))))))))

(event Custom|Move%20There
  (params (Move%20target :type Vector))
  ;[1 1 1] Move There Commands
  (Variables|Default|SetActive%20Command "NewEnumerator2")
  (AI|AIMoveTo self Move%20target 0 5e+02 false))

(event EventBeginPlay
  (bind _asbp_mush_player_b (Utilities|Casting|CastToBP_Mush_PlayerB (Game|GetPlayerCharacter 0)))
  (Variables|Default|SetChar%20REF _asbp_mush_player_b)
  (CallFunction|FollowPlayer))

(event Collision|EventActorBeginOverlap
  (params (OtherActor :type Actor%20Object%20Reference)))

(event EventTick
  (params (DeltaSeconds :type Float%20%28single-precision%29)))

(fn ConstructionScript)