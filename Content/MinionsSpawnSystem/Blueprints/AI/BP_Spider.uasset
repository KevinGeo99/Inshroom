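; BP_Spider is a spider character in the minion spawn system that takes damage and dies.
; On BeginPlay it caches the movement component's max walk speed in OriginSpeed, which this graph does not read again.
; AnyDamage subtracts from Health with a floor of zero, and an IsDead flag guards a single DestroyActor call when Health runs out.
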(event Game|Damage|EventAnyDamage
  (params (Damage :type Float%20%28single-precision%29) (DamageType :type Damage%20Type%20Object%20Reference) (InstigatedBy :type Controller%20Object%20Reference) (DamageCauser :type Actor%20Object%20Reference))
  ;[1 1 1] Any Damage
  (bind _output_get (Variables|Default|SetHealth (Math|Float|Max(Float) (+ (Variables|Default|GetHealth) (* Damage -1.0)) 0.0)))
  (if (and (== _output_get 0.0) (not (Variables|Default|GetIsDead)))
    (Variables|Default|SetIsDead true)
    (Actor|DestroyActor)))

(event EventBeginPlay
  (Variables|Default|SetOriginSpeed (Variables|/Script/Engine.CharacterMovementComponent|GetMaxWalkSpeed (Variables|Character|GetCharacterMovement))))

(fn ConstructionScript)