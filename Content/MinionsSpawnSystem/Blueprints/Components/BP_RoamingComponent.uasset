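; Roaming component for minions that makes its owning pawn wander via AI navigation around an origin point.
; The origin is the instigator's location, refreshed before each new target, or the owner's start location when it has no separate instigator.
; It picks a random reachable point within the roaming radius and re-issues MoveTo on a looping timer until arrival, then waits before repeating.
; Stop halts movement and clears both timers.
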(event Custom|-Start
  (bind _returnvalue (Components|GetOwner))
  (bind _instigator (Variables|/Script/Engine.Actor|GetInstigator _returnvalue)
    (:then
      (if (== _instigator _returnvalue)
        (Variables|DONOTTOUCH|SetOriginLocation (Transformation|GetActorLocation (Components|GetOwner)) :!label _label)
        (else
          (Variables|DONOTTOUCH|SetOriginLocation (Transformation|GetActorLocation _instigator)))))
    (:else
      (goto _label)))
  (CallFunction|-GotoNewTarget))

(event Custom|-Stop
  (bind _aspawn (Utilities|Casting|CastToPawn (Components|GetOwner)))
  (Components|Movement|StopMovementImmediately (Pawn|GetMovementComponent _aspawn))
  (Utilities|Time|ClearandInvalidateTimerbyHandle (Variables|DONOTTOUCH|GetTimer-MoveToLocation))
  (Utilities|Time|ClearandInvalidateTimerbyHandle (Variables|DONOTTOUCH|GetTimer-GoToNewTarget)))

(fn -GotoNewTarget
  (bind _returnvalue (Components|GetOwner))
  (bind _instigator (Variables|/Script/Engine.Actor|GetInstigator _returnvalue)
    (:then
      (if (== _instigator _returnvalue)
        _
        (else
          (Variables|DONOTTOUCH|SetOriginLocation (Transformation|GetActorLocation _instigator)))))
    (:else
      _))
  (bind _targetlocation (CallFunction|-FindLocation))
  (Variables|DONOTTOUCH|SetTargetLocation _targetlocation)
  (bind _returnvalue_2 (Utilities|Time|SetTimerbyFunctionName 0 "-MoveToLocation" 0.5 true))
  (Variables|DONOTTOUCH|SetTimer-MoveToLocation _returnvalue_2))

(fn -FindLocation
  (return (.RandomLocation (AI|Navigation|GetRandomReachablePointinRadius (Variables|DONOTTOUCH|GetOriginLocation) (Variables|Default|GetRoamingRadius) 0 0))))

(fn -MovetoLocation
  (bind _returnvalue (AI|Navigation|MovetoLocation (AI|GetAIController (Components|GetOwner)) (Variables|DONOTTOUCH|GetTargetLocation) 5e+01 true true false true 0))
  (switch Utilities|FlowControl|Switch|SwitchonEPathFollowingRequestResult _returnvalue
    (:AlreadyAtGoal
      (CallFunction|-TargetReached))))

(fn -TargetReached
  (Utilities|Time|ClearandInvalidateTimerbyHandle (Variables|DONOTTOUCH|GetTimer-MoveToLocation))
  (bind _returnvalue (Utilities|Time|SetTimerbyFunctionName 0 "-GoToNewTarget" (Variables|Default|GetWaitingTime)))
  (Variables|DONOTTOUCH|SetTimer-GoToNewTarget _returnvalue))