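; Melee attack component that drives a spawn place's spawned pawn to chase and hit a target.
; A looping timer issues AI MoveTo until the target is within range of the spawn place (not the pawn), and calls Relax when it is invalid or dead.
; Attacks play random slot montages, freezing Character movement meanwhile, and apply damage through a delayed forward sphere trace.
; Random picks re-roll per use, so animation and timings can mismatch.
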(event Custom|-AttackAnim
  (params (Asset :type Anim%20Sequence%20Base%20Object%20Reference))
  ;[1 1 1] Attack Animation
  (CallFunction|-AttackAnimMulti Asset))

(event Custom|-AttackAnimMulti
  (params (Asset :type Anim%20Sequence%20Base%20Object%20Reference))
  ;[1 1 1] Attack Animation
  (bind _spawnedpawn (Variables|/Game/MinionsSpawnSystem/Blueprints/BP_SpawnPlace.BP_SpawnPlace_C|GetSpawnedPawn (Variables|Default|GetSpawnPlace))
    (:then
      (bind _ascharacter (Utilities|Casting|CastToCharacter _spawnedpawn)
        (:then
          (bind _returnvalue (Class|AnimInstance|PlaySlotAnimationasDynamicMontage (Components|SkeletalMesh|GetAnimInstance (Variables|/Script/Engine.Character|GetMesh _ascharacter)) Asset "DefaultSlot" 0.1 0.1 1.0 1 -1.0 0.0))
          (Variables|Default|SetAttackAnimTime (Variables|/Script/Engine.AnimSequenceBase|GetSequenceLength _returnvalue))
          (Variables|/Script/Engine.CharacterMovementComponent|SetRotationRate (Variables|/Script/Engine.Character|GetCharacterMovement _ascharacter) "0, 0, 0")
          (Variables|/Script/Engine.CharacterMovementComponent|SetMaxWalkSpeed (Variables|/Script/Engine.Character|GetCharacterMovement _ascharacter) 0.0)
          (Utilities|FlowControl|Delay (Variables|/Script/Engine.AnimSequenceBase|GetSequenceLength _returnvalue))
          (Variables|/Script/Engine.CharacterMovementComponent|SetRotationRate (Variables|/Script/Engine.Character|GetCharacterMovement _ascharacter) (Variables|Default|GetOriginRotationRate))
          (Variables|/Script/Engine.CharacterMovementComponent|SetMaxWalkSpeed (Variables|/Script/Engine.Character|GetCharacterMovement _ascharacter) (Variables|Default|GetOriginWalkSpeed)))
        (:CastFailed
          (Utilities|IsValid (Components|SkeletalMesh|GetAnimInstance (Actor|GetComponentbyClass _spawnedpawn "/Script/Engine.SkeletalMeshComponent"))
            (:Is%20Valid
              (Class|AnimInstance|PlaySlotAnimationasDynamicMontage (Components|SkeletalMesh|GetAnimInstance (Actor|GetComponentbyClass _spawnedpawn "/Script/Engine.SkeletalMeshComponent")) Asset "DefaultSlot" 0.1 0.1 1.0 1 -1.0 0.0))))))
    (:else)))

(event Custom|-TakeDamage
  (params (Duration :type Float%20%28single-precision%29))
  (bind _spawnplace (Variables|Default|GetSpawnPlace))
  ;[1 1 1] Delay Take Damage
  (Utilities|FlowControl|Delay Duration)
  (bind _spawnedpawn (Variables|/Game/MinionsSpawnSystem/Blueprints/BP_SpawnPlace.BP_SpawnPlace_C|GetSpawnedPawn (Variables|Default|GetSpawnPlace))
    (:then
      (bind _outhit (Collision|SphereTraceForObjects (Transformation|GetActorLocation _spawnedpawn) (+ (* (Transformation|GetActorForwardVector _spawnedpawn) (Utilities|Struct|BreakStr_PawnInfo (Variables|/Game/MinionsSpawnSystem/Blueprints/BP_SpawnPlace.BP_SpawnPlace_C|GetSpawnInfo (Variables|Default|GetSpawnPlace)))) (Transformation|GetActorLocation _spawnedpawn)) 5.0 (Utilities|Array|MakeArray "ObjectTypeQuery1" "ObjectTypeQuery2" "ObjectTypeQuery3") false (Utilities|Array|MakeArray _spawnplace (Variables|/Game/MinionsSpawnSystem/Blueprints/BP_SpawnPlace.BP_SpawnPlace_C|GetSpawnedPawn _spawnplace)) "None"))
      (if (== (.HitActor (Collision|BreakHitResult _outhit)) (Variables|Default|GetTarget))
        (Game|Damage|ApplyDamage (Variables|Default|GetTarget) (Utilities|Struct|BreakStr_PawnInfo (Variables|/Game/MinionsSpawnSystem/Blueprints/BP_SpawnPlace.BP_SpawnPlace_C|GetSpawnInfo (Variables|Default|GetSpawnPlace))) 0 (Variables|/Game/MinionsSpawnSystem/Blueprints/BP_SpawnPlace.BP_SpawnPlace_C|GetSpawnedPawn (Variables|Default|GetSpawnPlace)))))
    (:else)))

(event Custom|-Init
  (params (SpawnPlace :type BP%20Spawn%20Place%20Object%20Reference))
  (bind _output_get (Variables|Default|SetSpawnPlace SpawnPlace))
  (Utilities|FlowControl|Delay 0.2)
  (bind _spawnedpawn (Variables|/Game/MinionsSpawnSystem/Blueprints/BP_SpawnPlace.BP_SpawnPlace_C|GetSpawnedPawn _output_get)
    (:then
      (bind _ascharacter (Utilities|Casting|CastToCharacter _spawnedpawn))
      (Variables|Default|SetOriginWalkSpeed (Variables|/Script/Engine.CharacterMovementComponent|GetMaxWalkSpeed (Variables|/Script/Engine.Character|GetCharacterMovement _ascharacter)))
      (Variables|Default|SetOriginRotationRate (Variables|/Script/Engine.CharacterMovementComponent|GetRotationRate (Variables|/Script/Engine.Character|GetCharacterMovement _ascharacter))))
    (:else)))

(event Custom|-Start
  (params (Target :type Actor%20Object%20Reference))
  (Variables|Default|SetTarget Target)
  (Variables|Default|SetAttack true)
  (bind _returnvalue (Utilities|Time|SetTimerbyFunctionName 0 "-MoveTo" 0.1 true))
  (Variables|Default|SetTimer-MoveTo _returnvalue))

(event Custom|-Stop
  (Utilities|Time|ClearandInvalidateTimerbyHandle (Variables|Default|GetTimer-MoveTo))
  (Variables|Default|SetTarget 0)
  (Variables|Default|SetAttack false))

(fn -Moveto
  (bind _target (Variables|Default|GetTarget)
    (:then
      (bind _spawnplace (Variables|Default|GetSpawnPlace)
        (:then
          (bind _spawnedpawn (Variables|/Game/MinionsSpawnSystem/Blueprints/BP_SpawnPlace.BP_SpawnPlace_C|GetSpawnedPawn _spawnplace)
            (:then
              (if (Variables|/Game/MinionsSpawnSystem/Blueprints/Components/BP_HealthComponent.BP_HealthComponent_C|GetIsDead (Actor|GetComponentbyClass _target "/Game/MinionsSpawnSystem/Blueprints/Components/BP_HealthComponent.BP_HealthComponent_C"))
                (Default|-Relax (Variables|Default|GetSpawnPlace))
                (elif (< (Math|Vector|Distance(Vector) (Transformation|GetActorLocation _spawnplace) (Transformation|GetActorLocation (Variables|Default|GetTarget))) (.DistancetoStartAttack (Utilities|Struct|BreakStr_PawnInfo (Variables|/Game/MinionsSpawnSystem/Blueprints/BP_SpawnPlace.BP_SpawnPlace_C|GetSpawnInfo (Variables|Default|GetSpawnPlace)))))
                  (CallFunction|-TargetReached)
                  (else
                    (AI|Navigation|MovetoActor (AI|GetAIController _spawnedpawn) (Variables|Default|GetTarget) -1.0 true true true 0)))))
            (:else)))
        (:else)))
    (:else
      (Default|-Relax (Variables|Default|GetSpawnPlace)))))

(fn -TargetReached
  (Utilities|Time|ClearandInvalidateTimerbyHandle (Variables|Default|GetTimer-MoveTo))
  (bind _spawnedpawn (Variables|/Game/MinionsSpawnSystem/Blueprints/BP_SpawnPlace.BP_SpawnPlace_C|GetSpawnedPawn (Variables|Default|GetSpawnPlace))
    (:then
      (Components|Movement|StopMovementImmediately (Pawn|GetMovementComponent _spawnedpawn))
      (Transformation|SetActorRelativeRotation _spawnedpawn (Math|Rotator|MakeRotator 0.0 0.0 (.Yaw (Math|Rotator|BreakRotator (Math|Rotator|FindLookatRotation (Transformation|GetActorLocation _spawnedpawn) (Transformation|GetActorLocation (Variables|Default|GetTarget)))))))
      (CallFunction|-Attack))
    (:else)))

(fn -Attack
  (bind _spawnplace (Variables|Default|GetSpawnPlace))
  (bind _spawninfo (Variables|/Game/MinionsSpawnSystem/Blueprints/BP_SpawnPlace.BP_SpawnPlace_C|GetSpawnInfo _spawnplace))
  (bind _attackanimations (Utilities|Struct|BreakStr_PawnInfo _spawninfo))
  (bind _returnvalue (Utilities|Array|LastIndex _attackanimations))
  (bind _returnvalue_2 (Math|Random|RandomIntegerinRange 0 _returnvalue))
  (bind _output (Utilities|Array|Get(acopy) _attackanimations _returnvalue_2))
  (bind (_animation _timetoadddamagetrace) (Utilities|Struct|BreakStr_AttackInfo _output))
  (Variables|Default|GetTarget
    (:then
      (if (> (Utilities|Array|Length _attackanimations) 0)
        (LocalVariables|Setlocal_AnimInfo _output)
        (Utilities|IsValid _animation
          (:Is%20Valid
            (CallFunction|-AttackAnim _animation)
            (CallFunction|-TakeDamage _timetoadddamagetrace)
            (bind _returnvalue_3 (Utilities|Time|SetTimerbyFunctionName 0 "-MoveTo" (Variables|/Script/Engine.AnimSequenceBase|GetSequenceLength _animation) true))
            (Variables|Default|SetTimer-MoveTo _returnvalue_3))
          (:Is%20Not%20Valid
            (bind _returnvalue_4 (Utilities|Time|SetTimerbyFunctionName 0 "-MoveTo" 1.0 true :!label _label))
            (Variables|Default|SetTimer-MoveTo _returnvalue_4)
            (CallFunction|-TakeDamage 1.0)))
        (else
          (goto _label))))
    (:else
      (CallFunction|-Stop))))