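; BP_HealthComponent is a health component in the minions spawn system that tracks current health and death.
; It starts at MaxHealth on BeginPlay, and UpdateHealth adds a signed delta, clamped at zero but with no upper limit.
; On first reaching zero it sets IsDead and calls HealthOver, with the flag preventing repeat notifications.
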(event EventBeginPlay
  (Variables|Default|SetCurrentHealth (Variables|Default|GetMaxHealth)))

(fn -UpdateHealth
  (params (Health :type Float%20%28double-precision%29))
  (bind _output_get (Variables|Default|SetCurrentHealth (Math|Float|Max(Float) (+ (Variables|Default|GetCurrentHealth) Health) 0.0)))
  (if (and (== _output_get 0.0) (not (Variables|Default|GetIsDead)))
    (Variables|Default|SetIsDead true)
    (Default|CallHealthOver)))