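; Melee attack component that makes its owner, typically a minion, chase and repeatedly strike a target.
; A looping timer drives AI MoveTo until in range, then the owner faces the target and plays a random attack montage, freezing Character movement meanwhile.
; A delayed forward sphere trace applies damage only if it hits the target, and the timer resumes the cycle.
; Dead or invalid targets trigger the minion component's Relax, or Stop without one.
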(event Custom|-AttackAnim
  (params (Asset :type Anim%20Sequence%20Base%20Object%20Reference))
  ;[1 1 1] Attack Animation
  (CallFunction|-AttackAnimMulti Asset))

(event Custom|-AttackAnimMulti
  (params (Asset :type Anim%20Sequence%20Base%20Object%20Reference))
  (bind _returnvalue (Components|GetOwner))
  (bind _returnvalue_2 (Actor|GetComponentbyClass _returnvalue "/Script/Engine.SkeletalMeshComponent"))
  (bind _returnvalue_3 (Components|SkeletalMesh|GetAnimInstance _returnvalue_2))
  ;[1 1 1] Attack Animation
  (bind _ascharacter (Utilities|Casting|CastToCharacter _returnvalue)
    (:then
      (bind _returnvalue_4 (Class|AnimInstance|PlaySlotAnimationasDynamicMontage (Components|SkeletalMesh|GetAnimInstance (Variables|/Script/Engine.Character|GetMesh _ascharacter)) Asset "DefaultSlot" 0.1 0.1 1.0 1 -1.0 0.0))
      (Variables|/Script/Engine.CharacterMovementComponent|SetRotationRate (Variables|/Script/Engine.Character|GetCharacterMovement _ascharacter) "0, 0, 0")
      (Variables|/Script/Engine.CharacterMovementComponent|SetMaxWalkSpeed (Variables|/Script/Engine.Character|GetCharacterMovement _ascharacter) 0.0)
      (Utilities|FlowControl|Sequence
        (:then_0
          (Utilities|FlowControl|Delay (Variables|/Script/Engine.AnimSequenceBase|GetSequenceLength _returnvalue_4))
          (Variables|/Script/Engine.CharacterMovementComponent|SetRotationRate (Variables|/Script/Engine.Character|GetCharacterMovement _ascharacter) (Variables|DONOTTOUCH|GetOriginRotationRate))
          (Variables|/Script/Engine.CharacterMovementComponent|SetMaxWalkSpeed (Variables|/Script/Engine.Character|GetCharacterMovement _ascharacter) (Variables|DONOTTOUCH|GetOriginWalkSpeed)))))
    (:CastFailed
      (Utilities|IsValid _returnvalue_3
        (:Is%20Valid
          (Class|AnimInstance|PlaySlotAnimationasDynamicMontage _returnvalue_3 Asset "DefaultSlot" 0.1 0.1 1.0 1 -1.0 0.0))))))

(event Custom|-TakeDamage
  (params (Duration :type Float%20%28single-precision%29))
  (bind _returnvalue (Components|GetOwner))
  (bind _returnvalue_2 (Transformation|GetActorLocation _returnvalue))
  ;[1 1 1] DelayTakeDamage
  (Utilities|FlowControl|Delay Duration)
  (bind _outhit (Collision|SphereTraceForObjects _returnvalue_2 (+ (* (Transformation|GetActorForwardVector _returnvalue) (Variables|Default|GetDistanceToStartAttack)) _returnvalue_2) 5.0 (Utilities|Array|MakeArray "ObjectTypeQuery1" "ObjectTypeQuery2" "ObjectTypeQuery3") false (Utilities|Array|MakeArray _returnvalue) "None"))
  (if (== (.HitActor (Collision|BreakHitResult _outhit)) (Variables|DONOTTOUCH|GetTarget))
    (Game|Damage|ApplyDamage (Variables|DONOTTOUCH|GetTarget) (Variables|Default|GetDamage) 0 (Components|GetOwner))))

(event Custom|-Start
  (params (Target :type Actor%20Object%20Reference))
  (Variables|DONOTTOUCH|SetTarget Target)
  (Variables|DONOTTOUCH|SetAttack true)
  (bind _returnvalue (Utilities|Time|SetTimerbyFunctionName 0 "-MoveTo" 0.1 true))
  (Variables|DONOTTOUCH|SetTimer-MoveTo _returnvalue))

(event Custom|-Stop
  (Utilities|Time|ClearandInvalidateTimerbyHandle (Variables|DONOTTOUCH|GetTimer-MoveTo))
  (Variables|DONOTTOUCH|SetTarget 0)
  (Variables|DONOTTOUCH|SetAttack false))

(event EventBeginPlay
  (Utilities|FlowControl|Delay 0.5)
  (bind _ascharacter (Utilities|Casting|CastToCharacter (Components|GetOwner)))
  (Variables|DONOTTOUCH|SetOriginWalkSpeed (Variables|/Script/Engine.CharacterMovementComponent|GetMaxWalkSpeed (Variables|/Script/Engine.Character|GetCharacterMovement _ascharacter)))
  (Variables|DONOTTOUCH|SetOriginRotationRate (Variables|/Script/Engine.CharacterMovementComponent|GetRotationRate (Variables|/Script/Engine.Character|GetCharacterMovement _ascharacter))))

(fn -Moveto
  (bind _returnvalue (Components|GetOwner))
  (bind _returnvalue_2 (Components|GetOwner))
  (bind _returnvalue_3 (Actor|GetComponentbyClass _returnvalue_2 "/Game/MinionsSpawnSystem/Blueprints/BP_MinionComponent.BP_MinionComponent_C"))
  (bind _target (Variables|DONOTTOUCH|GetTarget)
    (:then
      (Utilities|IsValid (Actor|GetComponentbyClass _target "/Game/MinionsSpawnSystem/Blueprints/Components/BP_HealthComponent.BP_HealthComponent_C")
        (:Is%20Valid
          (if (Variables|/Game/MinionsSpawnSystem/Blueprints/Components/BP_HealthComponent.BP_HealthComponent_C|GetIsDead (Actor|GetComponentbyClass _target "/Game/MinionsSpawnSystem/Blueprints/Components/BP_HealthComponent.BP_HealthComponent_C"))
            (Utilities|IsValid _returnvalue_3 :!label _label
              (:Is%20Valid
                (Default|-Relax _returnvalue_3))
              (:Is%20Not%20Valid
                (CallFunction|-Stop)))
            (else
              (if (< (Math|Vector|Distance(Vector) (Transformation|GetActorLocation _returnvalue) (Transformation|GetActorLocation (Variables|DONOTTOUCH|GetTarget))) (Variables|Default|GetDistanceToStartAttack)) :!label _label_2
                (CallFunction|-TargetReached)
                (else
                  (AI|Navigation|MovetoActor (AI|GetAIController _returnvalue) (Variables|DONOTTOUCH|GetTarget) -1.0 true true true 0))))))
        (:Is%20Not%20Valid
          (goto _label_2))))
    (:else
      (goto _label))))

(fn -TargetReached
  (bind _returnvalue (Components|GetOwner))
  (Utilities|Time|ClearandInvalidateTimerbyHandle (Variables|DONOTTOUCH|GetTimer-MoveTo))
  (Transformation|SetActorRelativeRotation _returnvalue (Math|Rotator|MakeRotator 0.0 0.0 (.Yaw (Math|Rotator|BreakRotator (Math|Rotator|FindLookatRotation (Transformation|GetActorLocation _returnvalue) (Transformation|GetActorLocation (Variables|DONOTTOUCH|GetTarget)))))))
  (CallFunction|-Attack))

(fn -Attack
  (bind _attackanim (Variables|Default|GetAttackAnim))
  (Variables|DONOTTOUCH|GetTarget
    (:then
      (if (> (Utilities|Array|Length _attackanim) 0)
        (bind _output_get (LocalVariables|Setlocal_RandomAttackAnim (Utilities|Array|Get(acopy) _attackanim (Math|Random|RandomIntegerinRange 0 (Utilities|Array|LastIndex _attackanim)))))
        (Utilities|IsValid (.Animation (Utilities|Struct|BreakStr_AttackInfo _output_get))
          (:Is%20Valid
            (CallFunction|-AttackAnim (.Animation (Utilities|Struct|BreakStr_AttackInfo _output_get)))
            (CallFunction|-TakeDamage (.TimeToAddDamageTrace (Utilities|Struct|BreakStr_AttackInfo _output_get)))
            (bind _returnvalue (Utilities|Time|SetTimerbyFunctionName 0 "-MoveTo" (Variables|/Script/Engine.AnimSequenceBase|GetSequenceLength (.Animation (Utilities|Struct|BreakStr_AttackInfo _output_get))) true))
            (Variables|DONOTTOUCH|SetTimer-MoveTo _returnvalue))
          (:Is%20Not%20Valid
            (bind _returnvalue_2 (Utilities|Time|SetTimerbyFunctionName 0 "-MoveTo" 1.0 true :!label _label))
            (Variables|DONOTTOUCH|SetTimer-MoveTo _returnvalue_2)
            (CallFunction|-TakeDamage 1.0)))
        (else
          (goto _label))))
    (:else
      (CallFunction|-Stop))))