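; Component in the minion spawn system that makes a minion wander randomly around a leader actor, or around itself when no leader is valid.
; Start picks a random reachable point within the roaming radius and sends the minion there through its AI controller.
; A looping timer re-issues the move until it reports already at goal, then a random-delay timer picks the next point.
; Stop clears both timers.
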(event Custom|-Start
  (CallFunction|-GotoNewTarget))

(event Custom|-Stop
  (Utilities|Time|ClearandInvalidateTimerbyHandle (Variables|DONOTTOUCH|GetTimer-MoveToLocation))
  (Utilities|Time|ClearandInvalidateTimerbyHandle (Variables|DONOTTOUCH|GetTimer-GoToNewTarget))
  (Variables|DONOTTOUCH|SetTargetLocation "0, 0, 0"))

(fn -GotoNewTarget
  (bind _leadertarget (Variables|DONOTTOUCH|GetLeaderTarget)
    (:then
      (Variables|DONOTTOUCH|SetLeaderLocation (Transformation|GetActorLocation _leadertarget))
      (bind _targetlocation (CallFunction|-FindLocation :!label _label))
      (Variables|DONOTTOUCH|SetTargetLocation _targetlocation)
      (CallFunction|-MovetoLocation)
      (bind _returnvalue (Utilities|Time|SetTimerbyFunctionName 0 "-MoveToLocation" 0.5 true))
      (Variables|DONOTTOUCH|SetTimer-MoveToLocation _returnvalue))
    (:else
      (bind _minionref (Variables|DONOTTOUCH|GetMinionRef)
        (:then
          (Variables|DONOTTOUCH|SetLeaderLocation (Transformation|GetActorLocation _minionref))
          (goto _label))
        (:else
          (CallFunction|-Stop))))))

(fn -FindLocation
  (return (.RandomLocation (AI|Navigation|GetRandomReachablePointinRadius (Variables|DONOTTOUCH|GetLeaderLocation) (Variables|Default|GetRoamingRadius) 0 0))))

(fn -MovetoLocation
  (bind _minionref (Variables|DONOTTOUCH|GetMinionRef)
    (:then
      (bind _returnvalue (AI|Navigation|MovetoLocation (AI|GetAIController _minionref) (Variables|DONOTTOUCH|GetTargetLocation) 5e+01 true true false true 0))
      (switch Utilities|FlowControl|Switch|SwitchonEPathFollowingRequestResult _returnvalue
        (:AlreadyAtGoal
          (CallFunction|-TargetReached))))
    (:else)))

(fn -TargetReached
  (Utilities|Time|ClearandInvalidateTimerbyHandle (Variables|DONOTTOUCH|GetTimer-MoveToLocation))
  (bind _returnvalue (Utilities|Time|SetTimerbyFunctionName 0 "-GoToNewTarget" (Math|Random|RandomFloatinRange (Variables|Default|GetWaitingTimeMin) (Variables|Default|GetWaitingTimeMax))))
  (Variables|DONOTTOUCH|SetTimer-GoToNewTarget _returnvalue))

(fn -Init
  (params (LeaderTarget :type Actor%20Object%20Reference) (MinionRef :type Pawn%20Object%20Reference) (RoamingRadius :type Float%20%28single-precision%29) (WaitingTime :type Float%20%28single-precision%29) (WaitingTimeMax :type Float%20%28single-precision%29))
  (Variables|DONOTTOUCH|SetLeaderTarget LeaderTarget)
  (Variables|DONOTTOUCH|SetMinionRef MinionRef)
  (Variables|Default|SetRoamingRadius RoamingRadius)
  (Variables|Default|SetWaitingTimeMin WaitingTime)
  (Variables|Default|SetWaitingTimeMax WaitingTimeMax))