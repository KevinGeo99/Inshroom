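; Actor component that turns its owner into the leader of a minion group with shared aggro.
; On Start it creates BP_SpawnPlace actors at random reachable points around the leader, each spawning and optionally respawning a minion.
; Damage events on leader and minions drive group aggro, switching from BP_RoamingComponent to BP_MeleeAttackComponent under the overridable default logic.
; A looping timer relaxes the leader when the target is invalid or too far.
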(event Custom|-SpawnPlaces
  (bind _returnvalue (Components|GetOwner))
  (bind _spawninfo (Variables|Default|GetSpawnInfo))
  (bind (_respawn_ _timetorespawn) (Utilities|Struct|BreakStr_SpawnInfo _spawninfo))
  ;[1 1 1] Spawn Places
  (Utilities|FlowControl|Delay 2.0)
  (Utilities|Array|Clear (Variables|DONOTTOUCH|GetSpawnPlaces))
  (for _array_element (Utilities|Struct|BreakStr_SpawnInfo (Variables|Default|GetSpawnInfo))
    (bind _output_get (Variables|DONOTTOUCH|SetCount (select (.RandomCount (Utilities|Struct|BreakStr_PawnInfo _array_element)) (Math|Random|RandomIntegerinRange (.Min (Utilities|Struct|BreakStr_PawnInfo _array_element)) (.Max (Utilities|Struct|BreakStr_PawnInfo _array_element))) (.Count (Utilities|Struct|BreakStr_PawnInfo _array_element)))))
    (for _index (range 0 (- _output_get 1))
      (bind _returnvalue_2 (Game|SpawnActorfromClass "/Game/MinionsSpawnSystem/Blueprints/BP_SpawnPlace.BP_SpawnPlace_C" (Math|Transform|MakeTransform (.RandomLocation (AI|Navigation|GetRandomReachablePointinRadius (Transformation|GetActorLocation _returnvalue) 3.5e+02 0 0)) "0, 0, 0" "1,1,1") "AdjustIfPossibleButAlwaysSpawn" _returnvalue _array_element _returnvalue _respawn_ _timetorespawn (Variables|Default|GetMinionRoamingRadius) (Variables|Default|GetWaitingTimeMin) (Variables|Default|GetWaitingTimeMax) (Variables|Default|GetDistanceToAbortPursuit) (Variables|Default|GetDefault_Minions_Agrr_Logic) (Variables|Default|GetMaxDistanceToArrive) self 0))
      (Utilities|Array|Add (Variables|DONOTTOUCH|GetSpawnPlaces) _returnvalue_2)
      (Default|-Spawn _returnvalue_2)))
  (for _array_element_2 (Variables|DONOTTOUCH|GetSpawnPlaces)
    (bind _spawnedpawn (Variables|/Game/MinionsSpawnSystem/Blueprints/BP_SpawnPlace.BP_SpawnPlace_C|GetSpawnedPawn _array_element_2)
      (:then
        (EventDispatchers|BindEventtoOnTakeAnyDamage _spawnedpawn (EventDispatchers|CreateEvent :!event -GroupAnyDamage)))
      (:else))))

(event Custom|-BindAnyDamage
  (params (SpawnedPawn :type Pawn%20Object%20Reference))
  ;[1 1 1] Bind Respawned Pawn
  (EventDispatchers|BindEventtoOnTakeAnyDamage SpawnedPawn (EventDispatchers|CreateEvent :!event -GroupAnyDamage)))

(event Custom|-Init
  ;[1 1 1] Init
  (CallFunction|-BindEvents))

(event Custom|-Start
  ;[1 1 1] Start
  (CallFunction|-Init)
  (CallFunction|-SpawnPlaces))

(event Custom|-Worried
  (params (Target :type Actor%20Object%20Reference))
  (bind _returnvalue (Components|GetOwner))
  (bind _returnvalue_2 (Actor|GetComponentbyClass _returnvalue "/Game/MinionsSpawnSystem/Blueprints/Components/BP_MeleeAttackComponent.BP_MeleeAttackComponent_C"))
  (bind _returnvalue_3 (Actor|GetComponentbyClass _returnvalue "/Game/MinionsSpawnSystem/Blueprints/Components/BP_RoamingComponent.BP_RoamingComponent_C"))
  ;[0.5781 0.06737 0 1 75] Worried and Relax Events for Leader. THIS DEFAULT. YOU CAN ADD YOU LOGIC
  (Utilities|IsValid Target
    (:Is%20Valid
      (Variables|DONOTTOUCH|SetCurrentTarget Target)
      (Variables|DONOTTOUCH|SetWorried true)
      (Utilities|FlowControl|Sequence
        (:then_0
          ;;[1 1 1] Stop Roaming
          (Utilities|IsValid _returnvalue_3
            (:Is%20Valid
              (Default|-Stop _returnvalue_3))))
        (:then_1
          (Utilities|IsValid _returnvalue_2
            (:Is%20Valid
              (Default|-Start _returnvalue_2 (Variables|DONOTTOUCH|GetCurrentTarget))
              (bind _returnvalue_4 (Utilities|Time|SetTimerbyFunctionName 0 "-CheckDistanceToAbortPursuit" 1.0 true))
              (Variables|DONOTTOUCH|SetTimer-CheckDistanceToAbortPursuit _returnvalue_4))))))))

(event Custom|-Relax
  (bind _returnvalue (Components|GetOwner))
  (bind _returnvalue_2 (Actor|GetComponentbyClass _returnvalue "/Game/MinionsSpawnSystem/Blueprints/Components/BP_RoamingComponent.BP_RoamingComponent_C"))
  (bind _returnvalue_3 (Actor|GetComponentbyClass _returnvalue "/Game/MinionsSpawnSystem/Blueprints/Components/BP_MeleeAttackComponent.BP_MeleeAttackComponent_C"))
  ;[0.5781 0.06737 0 1 75] Worried and Relax Events for Leader. THIS DEFAULT. YOU CAN ADD YOU LOGIC
  (Variables|DONOTTOUCH|SetCurrentTarget 0)
  (Variables|DONOTTOUCH|SetWorried false)
  (Utilities|IsValid _returnvalue_2
    (:Is%20Valid
      (Default|-Stop _returnvalue_3)
      (Utilities|IsValid _returnvalue_3
        (:Is%20Valid
          (Default|-Start _returnvalue_2)
          (Utilities|Time|ClearandInvalidateTimerbyHandle (Variables|DONOTTOUCH|GetTimer-CheckDistanceToAbortPursuit)))))))

(event Custom|-LeaderAggr
  (params (Target :type Actor%20Object%20Reference))
  (bind _returnvalue (Components|GetOwner))
  (bind _returnvalue_2 (Actor|GetComponentbyClass _returnvalue "/Game/MinionsSpawnSystem/Blueprints/Components/BP_RoamingComponent.BP_RoamingComponent_C"))
  ;[1 1 1] LEADER AGGR - Set YOU LOGIC
  (if (Variables|Default|GetDefault_Leader_Agrr_Logic)
    (CallFunction|-Worried Target)
    (else
      (Utilities|IsValid _returnvalue_2
        (:Is%20Valid
          (Default|-Stop _returnvalue_2))
        (:Is%20Not%20Valid)))))

(fn -BindEvents
  (EventDispatchers|BindEventtoOnTakeAnyDamage (Components|GetOwner) (EventDispatchers|CreateEvent :!event -GroupAnyDamage)))

(fn -GroupAnyDamage
  (params (DamagedActor :type Actor%20Object%20Reference) (Damage :type Float%20%28single-precision%29) (DamageType :type Damage%20Type%20Object%20Reference) (InstigatedBy :type Controller%20Object%20Reference) (DamageCauser :type Actor%20Object%20Reference))
  (for _array_element (Variables|DONOTTOUCH|GetSpawnPlaces)
    (bind _spawnedpawn (Variables|/Game/MinionsSpawnSystem/Blueprints/BP_SpawnPlace.BP_SpawnPlace_C|GetSpawnedPawn _array_element)
      (:then
        (Game|Damage|ApplyDamage _spawnedpawn 0.0 InstigatedBy DamageCauser)
        (Default|-Worried _array_element DamageCauser))
      (:else)))
  (Game|Damage|ApplyDamage (Components|GetOwner) 0.0 InstigatedBy DamageCauser)
  (CallFunction|-LeaderAggr DamageCauser))

(fn -CheckDistancetoAbortPursuit
  (bind _currenttarget (Variables|DONOTTOUCH|GetCurrentTarget)
    (:then
      (if (> (CallFunction|-GetDistancetoTargetAgrr _currenttarget) (Variables|Default|GetDistanceToAbortPursuit))
        (CallFunction|-Relax)))
    (:else
      (CallFunction|-Relax))))

(fn -GetDistancetoTargetAgrr
  (params (Target :type Actor%20Object%20Reference))
  (Utilities|IsValid Target
    (:Is%20Valid
      (return (Transformation|GetDistanceTo (Components|GetOwner) Target)))
    (:Is%20Not%20Valid
      (return 0.0))))