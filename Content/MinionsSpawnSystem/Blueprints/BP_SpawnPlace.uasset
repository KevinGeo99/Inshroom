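; BP_SpawnPlace spawns and manages one minion for a leader actor, attaching itself to the pawn and optionally respawning it on death while the leader lives.
; A roaming component wanders the minion around the leader, while a looping, randomly offset timer pulls it back when too far.
; When worried, it pursues a target through the default melee component or a behavior tree, relaxing once the target is lost or out of range.
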(event Custom|-Spawn
  (bind _spawninfo (Variables|Default|GetSpawnInfo))
  (bind _spawninfo_2 (Variables|Default|GetSpawnInfo))
  (bind _behaviortree (Utilities|Struct|BreakStr_PawnInfo _spawninfo_2))
  (bind (_pawnclass _scalemin _scalemax) (Utilities|Struct|BreakStr_PawnInfo _spawninfo))
  ;[1 1 1] Spawn Minion
  (bind _actorowner (Variables|Default|GetActorOwner)
    (:then
      (bind _returnvalue (Game|SpawnActorfromClass _pawnclass (Math|Transform|MakeTransform (.RandomLocation (Class|NavigationSystemV1|GetRandomPointinNavigableRadius (Transformation|GetActorLocation (Variables|Default|GetActorOwner)) 3.5e+02 0 0)) "0,0.000000, 0" (* (Transformation|GetActorScale3D _actorowner) (Math|Conversions|ToVector(Float) (Math|Random|RandomFloatinRange _scalemin _scalemax)))) "AdjustIfPossibleButAlwaysSpawn" 0 0))
      (bind _output_get (Variables|Default|SetSpawnedPawn _returnvalue))
      (Variables|/Game/MinionsSpawnSystem/Blueprints/Components/BP_RoamingPlaceComponent.BP_RoamingPlaceComponent_C|SetMinionRef (Variables|Default|GetBP_RoamingPlaceComponent) _output_get)
      (Utilities|IsValid _behaviortree
        (:Is%20Valid
          (AI|RunBehaviorTree (AI|GetAIController _output_get) _behaviortree))
        (:Is%20Not%20Valid
          _))
      (Game|BindEventtoOnDestroyed (Variables|Default|GetSpawnedPawn) (EventDispatchers|CreateEvent :!event Custom|-SpawnedPawnDestroyed))
      (Default|-BindAnyDamage (Variables|Default|GetOwnerMinionComponent) (Variables|Default|GetSpawnedPawn))
      (Transformation|AttachActorToActor (Variables|Default|GetSpawnedPawn) "None" "SnapToTarget" "SnapToTarget" "SnapToTarget" false)
      (CallFunction|BeginPlayServer))
    (:else)))

(event Custom|-Worried
  (params (Target :type Actor%20Object%20Reference))
  (bind _spawninfo (Variables|Default|GetSpawnInfo))
  (bind _behaviortree (Utilities|Struct|BreakStr_PawnInfo _spawninfo))
  ;[1 1 1] Worried and Relax Events
  (Utilities|IsValid Target
    (:Is%20Valid
      (Variables|Default|SetCurrentTarget Target)
      (Variables|Default|SetWorried true)
      (Default|-Stop (Variables|Default|GetBP_RoamingPlaceComponent))
      (bind _returnvalue (Utilities|Time|SetTimerbyFunctionName 0 "-CheckDistanceToAbortPursuit" 1.0 true))
      (Variables|Default|SetTimer-CheckDistanceToAbortPursuit _returnvalue)
      (if (Variables|Default|GetDEFAULT_MINIONS_AGRR_LOGIC)
        ;[1 0 0.04893 1 47] DEFAULT AGRR ATTACK LOGIC. REPLACE WITH YOU LOGIC.
        (Default|-Start (Variables|Default|GetBP_MeleeAttackSpawnPlaceComponent) (Variables|Default|GetCurrentTarget))
        (else
          ;;[0.1843 1 0] RUN BEHAVIOR TREE LOGIC
          (Utilities|IsValid _behaviortree
            (:Is%20Valid
              (AI|RunBehaviorTree (AI|GetAIController (Variables|Default|GetSpawnedPawn)) _behaviortree))))))))

(event Custom|-Relax
  ;[1 1 1] Worried and Relax Events
  (Variables|Default|SetCurrentTarget 0)
  (Variables|Default|SetWorried false)
  (Default|-Start (Variables|Default|GetBP_RoamingPlaceComponent))
  (Utilities|Time|ClearandInvalidateTimerbyHandle (Variables|Default|GetTimer-CheckDistanceToAbortPursuit))
  (Utilities|FlowControl|Sequence
    (:then_0
      (bind _bp_meleeattackspawnplacecomponent (Variables|Default|GetBP_MeleeAttackSpawnPlaceComponent)
        (:then
          (Default|-Stop _bp_meleeattackspawnplacecomponent))
        (:else)))
    (:then_1
      (if (not (Variables|Default|GetDEFAULT_MINIONS_AGRR_LOGIC))
        (AI|RunBehaviorTree (AI|GetAIController (Variables|Default|GetSpawnedPawn)))))))

(event Custom|-LeaderDestroyed
  (params (DestroyedActor :type Actor%20Object%20Reference))
  ;[1 1 1] Leader Destroyed = Stop Respawn
  (Utilities|Time|ClearandInvalidateTimerbyHandle (Variables|Default|GetTimer-Respawn)))

(event Custom|-SpawnedPawnDestroyed
  (params (DestroyedActor :type Actor%20Object%20Reference))
  ;[1 1 1] Respawn
  (Variables|Default|GetActorOwner
    (:then
      (if (Variables|Default|GetRespawn?)
        (bind _returnvalue (Utilities|Time|SetTimerbyFunctionName 0 "-Spawn" (Variables|Default|GetTimeToRespawn)))
        (Variables|Default|SetTimer-Respawn _returnvalue)
        (else
          (Actor|DestroyActor :!label _label))))
    (:else
      (goto _label))))

(event Custom|BeginPlay_Server
  (bind _bp_roamingplacecomponent (Variables|Default|GetBP_RoamingPlaceComponent))
  ;[1 1 1] Begin Play Server
  (Default|-Init _bp_roamingplacecomponent (Variables|Default|GetActorOwner) (Variables|Default|GetSpawnedPawn) (Variables|Default|GetRoamingRadius) (Variables|Default|GetWaitingTimeMin) (Variables|Default|GetWaitingTimeMax))
  (Variables|Default|SetRoaming true)
  (Default|-Start _bp_roamingplacecomponent)
  (bind _returnvalue (Utilities|Time|SetTimerbyFunctionName 0 "-CheckDistanceToLeader" (Math|Random|RandomFloatinRange 0.2 0.3) true))
  (Variables|Default|SetTimer-CheckDistanceToLeader _returnvalue)
  (Default|-Init (Variables|Default|GetBP_MeleeAttackSpawnPlaceComponent) self))

(fn ConstructionScript)

(fn -BindEvents
  (Game|BindEventtoOnDestroyed (Variables|Default|GetActorOwner) (EventDispatchers|CreateEvent :!event Custom|-LeaderDestroyed)))

(fn -GetDistancetoLeader
  (return (Transformation|GetDistanceTo (Variables|Default|GetActorOwner) (Variables|Default|GetSpawnedPawn))))

(fn -CheckDistancetoLeader
  (Variables|Default|GetActorOwner
    (:then
      (Variables|Default|GetSpawnedPawn
        (:then
          (if (not (Variables|Default|GetWorried))
            (if (> (CallFunction|-GetDistancetoLeader) (Variables|Default|GetMaxDistanceToArrive))
              (AI|Navigation|MovetoActor (AI|GetAIController (Variables|Default|GetSpawnedPawn)) (Variables|Default|GetActorOwner) 5e+01 true true true 0)
              (if (not (Variables|Default|GetReturn))
                (Default|-Stop (Variables|Default|GetBP_RoamingPlaceComponent))
                (Variables|Default|SetRoaming false)
                (Variables|Default|SetReturn true))
              (elif (not (Variables|Default|GetRoaming))
                (AI|Navigation|StopMovement (AI|GetAIController (Variables|Default|GetSpawnedPawn)))
                (Default|-Start (Variables|Default|GetBP_RoamingPlaceComponent))
                (Variables|Default|SetReturn false)
                (Variables|Default|SetRoaming true)))))
        (:else)))
    (:else)))

(fn -AttackCompleted
  (params (Target :type Actor%20Object%20Reference)))

(fn -GetDistancetoTarget
  (params (Target :type Actor%20Object%20Reference))
  (Utilities|IsValid Target
    (:Is%20Valid
      (bind _spawnedpawn (Variables|Default|GetSpawnedPawn)
        (:then
          (return (Transformation|GetDistanceTo Target _spawnedpawn)))
        (:else
          _)))
    (:Is%20Not%20Valid
      _))
  (return 0.0))

(fn -CheckDistancetoAbortPursuit
  (bind _currenttarget (Variables|Default|GetCurrentTarget)
    (:then
      (if (> (CallFunction|-GetDistancetoTarget _currenttarget) (Variables|Default|GetDistanceToAbortPursuit))
        (CallFunction|-Relax)))
    (:else
      (CallFunction|-Relax))))